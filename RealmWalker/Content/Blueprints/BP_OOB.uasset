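; BP_OOB is an out-of-bounds volume that returns the player or rolling crates to a set location when they overlap its collision box.
; The player character is teleported, while a BP_CrateRolling is destroyed and respawned fresh at double scale.
; CalculateNewTeleportLocation supplies both cases, converting the NewLocation transform's position from actor-relative to world space but using its rotation unconverted.
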(event OnComponentBeginOverlap(CollisionBox)
  (params (OverlappedComponent :type Primitive%20Component%20Object%20Reference) (OtherActor :type Actor%20Object%20Reference) (OtherComp :type Primitive%20Component%20Object%20Reference) (OtherBodyIndex :type Integer) (bFromSweep :type Boolean) (SweepResult :type Hit%20Result%20Structure%20%28by%20ref%29))
  (if (== OtherActor (Game|GetPlayerCharacter 0))
    (bind (_newtteleportvector _newteleportrotation) (CallFunction|CalculateNewTeleportLocation))
    (Transformation|SetActorLocationAndRotation OtherActor _newtteleportvector _newteleportrotation false true)
    (elif (== OtherActor (.AsBP%20Crate%20Rolling (Utilities|Casting|CastToBP_CrateRolling OtherActor)))
      (Actor|DestroyActor OtherActor)
      (bind (_newtteleportvector_2 _newteleportrotation_2) (CallFunction|CalculateNewTeleportLocation))
      (Game|SpawnActorfromClass "/Game/Blueprints/BP_CrateRolling.BP_CrateRolling_C" (Math|Transform|MakeTransform _newtteleportvector_2 _newteleportrotation_2 "2.000000,2.000000,2.000000") "Undefined" "MultiplyWithRoot" 0 0))))

(fn ConstructionScript)

(fn CalculateNewTeleportLocation
  (bind _new_location (Variables|Default|GetNew%20Location))
  (return (Math|Transform|TransformLocation (Transformation|GetActorTransform) (.location _new_location)) (.rotation _new_location)))