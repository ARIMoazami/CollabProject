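; BP_Door is a door that slides upward once three code checks have been registered.
; Each CodeCheck call increments IndicatorValue and fires OpenDoor when the count reaches exactly three.
; OpenDoor plays the Opening timeline from the start, lerping the Door component's relative location from the origin to a raised position along Z.
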(event Custom|OpenDoor
  (bind _alpha (Timeline|Opening PlayFromStart)
    (:Update
      (Transformation|SetRelativeLocation (Variables|Default|GetDoor) (Math|Vector|Lerp(Vector) "0, 0, 0" "0.000000,0.000000,400.000000" _alpha) false false))))

(event Custom|CodeCheck
  (bind _result (Math|Integer|IncrementInt (Variables|Default|GetIndicatorValue))
    (:%20%20
      (bind _output_get (Variables|Default|SetIndicatorValue _result))
      (if (== _output_get 3)
        (CallFunction|OpenDoor)))))

(fn ConstructionScript)