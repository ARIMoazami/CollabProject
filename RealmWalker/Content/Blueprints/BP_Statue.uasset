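; BP_Statue is an interactable statue that rotates and reports to a referenced Portal.
; Each Interact call snaps the Statue component's relative yaw forward 45 degrees, through a Lerp fixed at full alpha.
; When yaw exceeds 360, it resets the rotation and calls StatueCheck on the Portal with its Value.
; The Box overlap event and construction script are empty.
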(event OnComponentBeginOverlap(Box)
  (params (OverlappedComponent :type Primitive%20Component%20Object%20Reference) (OtherActor :type Actor%20Object%20Reference) (OtherComp :type Primitive%20Component%20Object%20Reference) (OtherBodyIndex :type Integer) (bFromSweep :type Boolean) (SweepResult :type Hit%20Result%20Structure%20%28by%20ref%29)))

(event EventInteract
  (params (Player :type BP%20First%20Person%20Character%20Object%20Reference))
  (Transformation|SetRelativeRotation (Variables|Default|GetStatue) (Math|Rotator|MakeRotator 0.0 0.0 (Math|Float|Lerp (.yaw (Variables|/Script/Engine.SceneComponent|GetRelativeRotation (Variables|Default|GetStatue))) (+ (.yaw (Variables|/Script/Engine.SceneComponent|GetRelativeRotation (Variables|Default|GetStatue))) 45.0) 1.0)) false false)
  (if (> (.yaw (Variables|/Script/Engine.SceneComponent|GetRelativeRotation (Variables|Default|GetStatue))) 3.6e+02)
    (Transformation|SetRelativeRotation (Variables|Default|GetStatue) (Math|Rotator|MakeRotator 0.0 0.0 0.0) false false)
    (Default|StatueCheck (Variables|Default|Getportal) (Variables|Default|GetValue))))

(fn ConstructionScript)