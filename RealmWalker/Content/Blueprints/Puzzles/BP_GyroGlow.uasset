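; BP_GyroGlow is an interactable puzzle actor that toggles a dissolve effect on its cube and the player's GyroActive state.
; The construction script creates a dynamic instance of MI_DissolveGryo on the cube.
; Each Interact alternates via FlipFlop between two timelines that lerp Dissolve Amount from its stored value toward opposite extremes.
; GyroActive turns on as the first timeline plays and off only when the reverse one finishes.
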(event EventInteract
  (params (Player :type BP%20First%20Person%20Character%20Object%20Reference))
  (Utilities|FlowControl|FlipFlop
    (:A
      (bind _alpha (Timeline|Timeline PlayFromStart)
        (:Update
          (Rendering|Material|SetScalarParameterValue (Variables|Default|GetDissolveMaterial) "Dissolve Amount" (Math|Float|Lerp (Variables|Default|GetCurrentDissolveValue) 1.0 _alpha) :!class /Script/Engine.MaterialInstanceDynamic)
          (Variables|/Game/FirstPerson/Blueprints/BP_FirstPersonCharacter.BP_FirstPersonCharacter_C|SetGyroActive? Player true))
        (:Finished
          (Variables|Default|SetCurrentDissolveValue (Math|Float|Lerp (Variables|Default|GetCurrentDissolveValue) 1.0 _alpha)))))
    (:B
      (bind _alpha_2 (Timeline|Timeline_0 PlayFromStart)
        (:Update
          (Rendering|Material|SetScalarParameterValue (Variables|Default|GetDissolveMaterial) "Dissolve Amount" (Math|Float|Lerp (Variables|Default|GetCurrentDissolveValue) -1.0 _alpha_2) :!class /Script/Engine.MaterialInstanceDynamic))
        (:Finished
          (Variables|Default|SetCurrentDissolveValue (Math|Float|Lerp (Variables|Default|GetCurrentDissolveValue) -1.0 _alpha_2))
          (Variables|/Game/FirstPerson/Blueprints/BP_FirstPersonCharacter.BP_FirstPersonCharacter_C|SetGyroActive? Player false))))))

(fn ConstructionScript
  (bind _returnvalue (Rendering|Material|CreateDynamicMaterialInstance (Variables|Default|GetCube) 0 "/Game/Materials/MI_DissolveGryo.MI_DissolveGryo" "None" :!class /Script/Engine.PrimitiveComponent))
  (Variables|Default|SetDissolveMaterial _returnvalue))