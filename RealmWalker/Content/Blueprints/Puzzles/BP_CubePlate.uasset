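; BP_CubePlate is a puzzle pressure plate that activates a linked Gate when a BP_CrateRolling overlaps its Box.
; Activation switches two cables to the lit material, calls Gate.OnPlate and optionally spawns another crate at the CubeSpawn point.
; End overlap calls Gate.OffPlate for any actor, leaving the cables lit.
; Each overlap handler runs only once, and the first overlap consumes its DoOnce before the crate check.
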(event OnComponentBeginOverlap(Box)
  (params (OverlappedComponent :type Primitive%20Component%20Object%20Reference) (OtherActor :type Actor%20Object%20Reference) (OtherComp :type Primitive%20Component%20Object%20Reference) (OtherBodyIndex :type Integer) (bFromSweep :type Boolean) (SweepResult :type Hit%20Result%20Structure%20%28by%20ref%29))
  (bind _cubespawn (Variables|Default|GetCubeSpawn))
  (Utilities|FlowControl|DoOnce false
    (:Completed
      (if (== OtherActor (.AsBP%20Crate%20Rolling (Utilities|Casting|CastToBP_CrateRolling OtherActor)))
        (Rendering|Material|SetMaterial (Variables|/Script/CableComponent.CableActor|GetCableComponent (Variables|Default|GetCable1)) 0 "/Game/Materials/M_CableOn.M_CableOn")
        (Default|OnPlate (Variables|Default|GetGate))
        (if (Variables|Default|GetSpawnCube?)
          (Game|SpawnActorfromClass "/Game/Blueprints/BP_CrateRolling.BP_CrateRolling_C" (Math|Transform|MakeTransform (Math|Transform|TransformLocation (Transformation|GetActorTransform) (.location _cubespawn)) (.rotation _cubespawn) "2.000000,2.000000,2.000000") "Undefined" "MultiplyWithRoot" 0 0))))))

(event OnComponentEndOverlap(Box)
  (params (OverlappedComponent :type Primitive%20Component%20Object%20Reference) (OtherActor :type Actor%20Object%20Reference) (OtherComp :type Primitive%20Component%20Object%20Reference) (OtherBodyIndex :type Integer))
  (Utilities|FlowControl|DoOnce false
    (:Completed
      (Default|OffPlate (Variables|Default|GetGate)))))

(fn ConstructionScript)