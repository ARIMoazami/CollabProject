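; Pressure plate puzzle actor that notifies a referenced Gate when something enters or leaves its Box trigger.
; Begin and end overlap set PlateActive, then call OnPlate or OffPlate on the Gate, with no filter on the overlapping actor.
; Each call has its own DoOnce that resets after a one-second delay, so repeat triggers within that window update only the flag.
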(event OnComponentBeginOverlap(Box)
  (params (OverlappedComponent :type Primitive%20Component%20Object%20Reference) (OtherActor :type Actor%20Object%20Reference) (OtherComp :type Primitive%20Component%20Object%20Reference) (OtherBodyIndex :type Integer) (bFromSweep :type Boolean) (SweepResult :type Hit%20Result%20Structure%20%28by%20ref%29))
  (Variables|Default|SetPlateActive? true)
  (Utilities|FlowControl|DoOnce false :!label _label
    (:Completed
      (Default|OnPlate (Variables|Default|GetGate))
      (Utilities|FlowControl|Delay 1.0)
      (goto _label Reset))))

(event OnComponentEndOverlap(Box)
  (params (OverlappedComponent :type Primitive%20Component%20Object%20Reference) (OtherActor :type Actor%20Object%20Reference) (OtherComp :type Primitive%20Component%20Object%20Reference) (OtherBodyIndex :type Integer))
  (Variables|Default|SetPlateActive? false)
  (Utilities|FlowControl|DoOnce false :!label _label
    (:Completed
      (Default|OffPlate (Variables|Default|GetGate))
      (Utilities|FlowControl|Delay 1.0)
      (goto _label Reset))))

(fn ConstructionScript)