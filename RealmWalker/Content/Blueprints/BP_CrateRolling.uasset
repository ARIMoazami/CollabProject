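; Interactable crate that the player rolls edge over edge in one of four directions, picked from the player's yaw, and outlines while the player overlaps its box.
; RollDirectional spawns a temporary BP_RotationPoint at a bottom edge and attaches the crate, then a timeline rotates that pivot.
; Four downward traces check the floor during and after each roll.
; Any miss switches on physics and applies torque so the crate topples.
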(event OnComponentBeginOverlap(Box)
  (params (OverlappedComponent :type Primitive%20Component%20Object%20Reference) (OtherActor :type Actor%20Object%20Reference) (OtherComp :type Primitive%20Component%20Object%20Reference) (OtherBodyIndex :type Integer) (bFromSweep :type Boolean) (SweepResult :type Hit%20Result%20Structure%20%28by%20ref%29))
  (if (== OtherActor (Game|GetPlayerCharacter 0))
    (CallFunction|ObjectHoveredOutline true (Variables|Default|GetCrate))))

(event OnComponentHit(Crate)
  (params (HitComponent :type Primitive%20Component%20Object%20Reference) (OtherActor :type Actor%20Object%20Reference) (OtherComp :type Primitive%20Component%20Object%20Reference) (NormalImpulse :type Vector :default "0, 0, 0") (Hit :type Hit%20Result%20Structure%20%28by%20ref%29)))

(event OnComponentEndOverlap(Box)
  (params (OverlappedComponent :type Primitive%20Component%20Object%20Reference) (OtherActor :type Actor%20Object%20Reference) (OtherComp :type Primitive%20Component%20Object%20Reference) (OtherBodyIndex :type Integer))
  (if (== OtherActor (Game|GetPlayerCharacter 0))
    (CallFunction|ObjectHoveredOutline false (Variables|Default|GetCrate))))

(event EventInteract
  (params (Player :type BP%20First%20Person%20Character%20Object%20Reference))
  (bind _returnvalue (Transformation|GetActorScale3D))
  (bind _crate (Variables|Default|GetCrate))
  (bind _floorspacebuffer (Variables|Default|GetFloorSpaceBuffer))
  (bind _cast_bounds_buffer (Variables|Default|GetCast%20Bounds%20Buffer))
  (bind _cube_timeline (Variables|Default|GetCube_Timeline))
  (bind _returnvalue_2 (Transformation|GetWorldLocation _crate))
  (bind _returnvalue_3 (Class|TimelineComponent|GetScaledTimelineLength _cube_timeline))
  (bind _returnvalue_4 (* "-25.000000,-25.000000,-25.000000" _returnvalue))
  (bind (_x _y _z) (Math|Vector|BreakVector _returnvalue_4))
  (bind _returnvalue_5 (+ _cast_bounds_buffer _y))
  (bind _returnvalue_6 (+ _z _floorspacebuffer))
  (bind _returnvalue_7 (+ _cast_bounds_buffer _x))
  (bind _returnvalue_8 (Math|Vector|MakeVector 0.0 _returnvalue_5 0.0))
  (bind _returnvalue_9 (Math|Vector|MakeVector 0.0 0.0 _returnvalue_6))
  (bind _returnvalue_10 (Math|Vector|MakeVector _returnvalue_7 0.0 0.0))
  (bind _returnvalue_11 (+ _returnvalue_9 _returnvalue_2))
  (if (== Player (Game|GetPlayerCharacter 0))
    (if (not (Variables|Default|GetIsAnimating))
      (Variables|Default|SetIsAnimating true)
      (bind _direction (CallFunction|GetPlayerDirection))
      (bind (_get_rolling_direction _rolling_actor) (CallFunction|RollDirectional _direction))
      (Utilities|FlowControl|Sequence
        (:then_0
          (bind _cube_rotation (Timeline|Cube_Timeline PlayFromStart)
            (:Update
              ;[1 1 1] Only neccesary if Physics is disabled
              (Transformation|SetActorRotation _rolling_actor (Math|Rotator|Lerp(Rotator) "0, 0, 0" _get_rolling_direction _cube_rotation)))
            (:Finished
              (Utilities|FlowControl|Delay 0.0)
              ;[1 1 1] Set Finished to Destroy Actor node only if Physics is disabled
              (Actor|DestroyActor _rolling_actor)
              (Variables|Default|SetIsAnimating false)
              (Variables|Default|SetCast_hits 0.0 :!label _label)
              (for (_array_element _array_index) (Utilities|Array|MakeArray (+ _returnvalue_11 _returnvalue_10) (- _returnvalue_11 _returnvalue_10) (+ _returnvalue_11 _returnvalue_8) (- _returnvalue_11 _returnvalue_8))
                (bind _returnvalue_12 (Collision|MultiLineTraceByChannel _array_element (Math|Vector|MakeVector (.X (Math|Vector|BreakVector _array_element)) (.Y (Math|Vector|BreakVector _array_element)) (- (.Z (Math|Vector|BreakVector _array_element)) 1e+02)) "TraceTypeQuery1" false 0 "ForOneFrame"))
                (if _returnvalue_12
                  (Development|PrintString (Utilities|String|Append "Ray" (Utilities|String|ToString(Integer) _array_index) "Hit"))
                  (Variables|Default|SetCast_hits (+ (Variables|Default|GetCast_hits) 1.0))
                  (else
                    (Development|PrintString (Utilities|String|Append "Ray" (Utilities|String|ToString(Integer) _array_index) "Miss")))))
              (if (< (Variables|Default|GetCast_hits) 4.0)
                (if (not (Variables|Default|GetPhysicsEnabled?))
                  (Physics|SetSimulatePhysics (Variables|Default|GetCrate) true)
                  (Variables|Default|SetPhysicsEnabled? true)
                  (bind _newtrack_0 (Timeline|FailForce PlayFromStart)
                    (:Update
                      (Class|PrimitiveComponent|AddTorqueinRadians (Variables|Default|GetCrate) (Math|Vector|MakeVector (.Roll (Math|Rotator|BreakRotator (Math|Rotator|Lerp(Rotator) "0, 0, 0" (* _get_rolling_direction -0.25) _newtrack_0))) (.Pitch (Math|Rotator|BreakRotator (Math|Rotator|Lerp(Rotator) "0, 0, 0" (* _get_rolling_direction -0.25) _newtrack_0))) (.Yaw (Math|Rotator|BreakRotator (Math|Rotator|Lerp(Rotator) "0, 0, 0" (* _get_rolling_direction -0.25) _newtrack_0)))) "None" true))))))))
        (:then_1
          (Utilities|FlowControl|Delay (/ _returnvalue_3 1.5))
          (goto _label))
        (:then_2
          (Utilities|FlowControl|Delay (/ _returnvalue_3 2.5))
          (goto _label))))))

(event EventBeginPlay
  (Components|Timeline|SetPlayRate (Variables|Default|GetCube_Timeline) (Variables|Default|GetPlayRate)))

(fn ConstructionScript)

(fn RollDirectional
  (params (Direction :type E_RotationDirection%20Enum :default "NewEnumerator0"))
  (bind _returnvalue (Transformation|GetActorScale3D))
  (bind _crate (Variables|Default|GetCrate))
  (bind _roll_amount (LocalVariables|GetRoll_Amount))
  (bind _roll_amount_2 (LocalVariables|GetRoll_Amount))
  (bind _returnvalue_2 (Transformation|GetWorldLocation _crate))
  (bind _returnvalue_3 (* "-25.000000,-25.000000,-25.000000" _returnvalue))
  (bind (_x _y _z) (Math|Vector|BreakVector _returnvalue_3))
  (bind _returnvalue_4 (Math|Vector|MakeVector 0.0 _y 0.0))
  (bind _returnvalue_5 (Math|Vector|MakeVector 0.0 0.0 _z))
  (bind _returnvalue_6 (Math|Vector|MakeVector _x 0.0 0.0))
  (bind _returnvalue_7 (+ _returnvalue_5 _returnvalue_2))
  (switch Utilities|FlowControl|Switch|SwitchonE_RotationDirection Direction
    (:NewEnumerator0
      (LocalVariables|SetRolling_Point (+ _returnvalue_7 _returnvalue_6))
      (LocalVariables|SetRolling_Direction (Math|Rotator|MakeRotator 0.0 _roll_amount_2 0.0)))
    (:NewEnumerator1
      (LocalVariables|SetRolling_Point (+ _returnvalue_7 _returnvalue_4))
      (LocalVariables|SetRolling_Direction (Math|Rotator|MakeRotator (- 0.0 _roll_amount) 0.0 0.0)))
    (:NewEnumerator2
      (LocalVariables|SetRolling_Point (- _returnvalue_7 _returnvalue_6))
      (LocalVariables|SetRolling_Direction (Math|Rotator|MakeRotator 0.0 (- 0.0 _roll_amount_2) 0.0)))
    (:NewEnumerator3
      (LocalVariables|SetRolling_Point (- _returnvalue_7 _returnvalue_4))
      (LocalVariables|SetRolling_Direction (Math|Rotator|MakeRotator _roll_amount 0.0 0.0))))
  ;[1 1 1] Only neccessary if physics is disabled
  (bind _returnvalue_8 (Game|SpawnActorfromClass "/Game/Blueprints/BP_RotationPoint.BP_RotationPoint_C" (Math|Transform|MakeTransform (LocalVariables|GetRolling_Point) "0, 0, 0" "1.000000,1.000000,1.000000") "Undefined" "MultiplyWithRoot" 0 0))
  (Transformation|AttachActorToActor _returnvalue_8 "None" "KeepWorld" "KeepWorld" "KeepWorld" true)
  (return (LocalVariables|GetRolling_Direction) _returnvalue_8))

(fn GetPlayerDirection
  (bind _returnvalue (Game|GetPlayerCharacter 0))
  (bind _returnvalue_2 (Transformation|GetActorRotation _returnvalue))
  (bind _yaw (Math|Rotator|BreakRotator _returnvalue_2))
  (if (>= _yaw 135.0)
    _
    (elif (>= _yaw 45.0)
      (return "NewEnumerator3")
      (elif (>= _yaw -45.0)
        (return "NewEnumerator2")
        (elif (<= _yaw -135.0)
          _
          (else
            (return "NewEnumerator1"))))))
  (return "NewEnumerator0"))