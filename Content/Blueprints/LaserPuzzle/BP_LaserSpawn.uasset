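; Laser puzzle emitter that spawns the first BP_Laser at its Arrow on BeginPlay and tracks lasers in ChildLasers.
; The spawned laser takes the spawner's display name as its ID, plus its colour and a back-reference to the spawner.
; RemoveFollowingLasers walks the list backwards, calls CancelTargetHit on lasers whose ID contains the given laser's ID, and drops those returning true.
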(event EventBeginPlay
  (Variables|Default|SetSpawnReference self)
  (Variables|Default|SetID (Utilities|GetDisplayName self))
  (bind _returnvalue (Game|SpawnActorfromClass "/Game/Blueprints/LaserPuzzle/BP_Laser.BP_Laser_C" (Math|Transform|MakeTransform (Transformation|GetWorldLocation (Variables|Default|GetArrow)) (Transformation|GetActorRotation) "1.000000,1.000000,1.000000") "Undefined" "MultiplyWithRoot" 0 (Variables|Default|GetID) (Variables|Default|GetLaserColour) (Variables|Default|GetSpawnReference) 0))
  (Utilities|Array|Add (Variables|Default|GetChildLasers) _returnvalue))

(fn ConstructionScript
  (|CallParentFunction))

(fn RemoveFollowingLasers
  (params (Laser%20Reference :type BP%20Laser%20Object%20Reference))
  (LocalVariables|SetLaser%20ID%20Removed (Variables|/Game/Blueprints/LaserPuzzle/BP_Laser.BP_Laser_C|GetLaserID Laser%20Reference))
  (bind _arrayelement (Utilities|Array|ReverseforEachLoop (Variables|Default|GetChildLasers))
    (:LoopBody
      (Utilities|IsValid _arrayelement
        (:Is%20Valid
          (if (Utilities|String|Contains (Variables|/Game/Blueprints/LaserPuzzle/BP_Laser.BP_Laser_C|GetLaserID _arrayelement) (LocalVariables|GetLaser%20ID%20Removed))
            (bind _removefromarray (Default|CancelTargetHit _arrayelement (Utilities|Enum|Equal(Enum) (Variables|/Game/Blueprints/LaserPuzzle/BP_Laser.BP_Laser_C|GetLaserID _arrayelement) (LocalVariables|GetLaser%20ID%20Removed))))
            (if _removefromarray
              (Utilities|Array|RemoveItem (Variables|Default|GetChildLasers) _arrayelement))))))))