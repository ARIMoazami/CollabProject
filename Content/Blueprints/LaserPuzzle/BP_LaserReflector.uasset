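; BP_LaserReflector is a laser puzzle piece that bounces lasers hitting it.
; On a hit, LaserBounce spawns a BP_Laser at the impact point, aligning its Z axis to the incoming direction mirrored about the surface normal.
; The new laser inherits colour and spawn reference, gets an updated ID, and is tracked here and in the source's child lasers.
; Without a hit response, attached lasers whose ID contains the incoming laser's ID are destroyed.
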(event EventBeginPlay)

(event Collision|EventActorBeginOverlap
  (params (OtherActor :type Actor%20Object%20Reference)))

(event EventTick
  (params (DeltaSeconds :type Float%20%28single-precision%29)))

(fn ConstructionScript
  (|CallParentFunction))

(fn ClearAttachedLasers
  (params (ID%20Clear :type String))
  (bind _arrayelement (Utilities|Array|ReverseforEachLoop (Variables|Default|GetLasersAttached))
    (:LoopBody
      (Utilities|IsValid _arrayelement
        (:Is%20Valid
          (if (Utilities|String|Contains (Variables|/Game/Blueprints/LaserPuzzle/BP_Laser.BP_Laser_C|GetLaserID _arrayelement) ID%20Clear)
            (Actor|DestroyActor _arrayelement)
            (Utilities|Array|RemoveItem (Variables|/Game/Blueprints/LaserPuzzle/BP_LaserStatue.BP_LaserStatue_C|GetLasersAttached _arrayelement) _arrayelement)))))))

(fn CalculateRotation
  (params (ImpactPoint :type Vector) (ImpactNormal :type Vector) (TraceStart :type Vector))
  (return (Math|Rotator|MakeRotfromZ (Math|Vector|MirrorVectorbyNormal (- ImpactPoint TraceStart) ImpactNormal))))

(fn LaserBounce
  (params (LaserHit :type BP%20Laser%20Object%20Reference) (HitResponse :type Boolean) (HitInformation :type Hit%20Result%20Structure))
  (bind (_bblockinghit _binitialoverlap _time _distance _location _impactpoint _normal _impactnormal _physmat _hitactor _hitcomponent _hitbonename _bonename _hititem _elementindex _faceindex _tracestart) (Collision|BreakHitResult HitInformation))
  (if HitResponse
    (bind _returnvalue (Game|SpawnActorfromClass "/Game/Blueprints/LaserPuzzle/BP_Laser.BP_Laser_C" (Math|Transform|MakeTransform _impactpoint (CallFunction|CalculateRotation _impactpoint _impactnormal _tracestart) "1.000000,1.000000,1.000000") "Undefined" "MultiplyWithRoot" 0 (Default|UpdateID LaserHit "B") (Variables|/Game/Blueprints/LaserPuzzle/BP_LaserStatue.BP_LaserStatue_C|GetLaserColour LaserHit) (Variables|/Game/Blueprints/LaserPuzzle/BP_LaserStatue.BP_LaserStatue_C|GetSpawnReference LaserHit) 0))
    (Utilities|Array|Add (Variables|Default|GetLasersAttached) _returnvalue)
    (Utilities|Array|Add (Variables|/Game/Blueprints/LaserPuzzle/BP_LaserSpawn.BP_LaserSpawn_C|GetChildLasers (Variables|/Game/Blueprints/LaserPuzzle/BP_LaserStatue.BP_LaserStatue_C|GetSpawnReference LaserHit)) _returnvalue)
    (return _returnvalue)
    (else
      (CallFunction|ClearAttachedLasers (Variables|/Game/Blueprints/LaserPuzzle/BP_Laser.BP_Laser_C|GetLaserID LaserHit)))))