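; Laser puzzle cube that redirects an incoming laser along its arrow and can be rotated in 45-degree yaw steps by interaction.
; A box trigger outlines the mesh while the player overlaps it.
; On a new hit, LaserBounce spawns an attached child BP_Laser with the incoming colour and an updated ID, registering it with the incoming laser's SpawnReference.
; Losing the hit clears all lasers.
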(event OnComponentBeginOverlap(Box)
  (params (OverlappedComponent :type Primitive%20Component%20Object%20Reference) (OtherActor :type Actor%20Object%20Reference) (OtherComp :type Primitive%20Component%20Object%20Reference) (OtherBodyIndex :type Integer) (bFromSweep :type Boolean) (SweepResult :type Hit%20Result%20Structure%20%28by%20ref%29))
  (if (== OtherActor (Game|GetPlayerCharacter 0))
    (CallFunction|ObjectHoveredOutline true (Variables|Character|GetMesh))))

(event OnComponentEndOverlap(Box)
  (params (OverlappedComponent :type Primitive%20Component%20Object%20Reference) (OtherActor :type Actor%20Object%20Reference) (OtherComp :type Primitive%20Component%20Object%20Reference) (OtherBodyIndex :type Integer))
  (if (== OtherActor (Game|GetPlayerCharacter 0))
    (CallFunction|ObjectHoveredOutline false (Variables|Character|GetMesh))))

(event EventInteract
  (params (Player :type BP%20First%20Person%20Character%20Object%20Reference))
  (Transformation|SetActorRotation (Math|Rotator|MakeRotator 0.0 0.0 (+ (Variables|Default|GetRotation) 45.0)))
  (Variables|Default|SetRotation (+ (Variables|Default|GetRotation) 45.0)))

(fn ConstructionScript
  (|CallParentFunction))

(fn LaserBounce
  (params (LaserHit :type BP%20Laser%20Object%20Reference) (HitResponse :type Boolean) (HitInformation :type Hit%20Result%20Structure))
  (bind _arrow (Variables|Default|GetArrow))
  (Utilities|IsValid LaserHit
    (:Is%20Valid
      (Variables|Default|SetSpawnReference (Variables|/Game/Blueprints/LaserPuzzle/BP_LaserStatue.BP_LaserStatue_C|GetSpawnReference LaserHit))
      (if (or (and HitResponse (not (Variables|Default|GetActive?))) (not HitResponse))
        (bind _output_get (Variables|Default|SetActive? HitResponse))
        (if _output_get
          (bind _returnvalue (Game|SpawnActorfromClass "/Game/Blueprints/LaserPuzzle/BP_Laser.BP_Laser_C" (Math|Transform|MakeTransform (Transformation|GetWorldLocation _arrow) (Math|Rotator|MakeRotfromZ (Math|Vector|GetForwardVector _arrow)) "1.000000,1.000000,1.000000") "Undefined" "MultiplyWithRoot" 0 (Default|UpdateID LaserHit "C") (Variables|/Game/Blueprints/LaserPuzzle/BP_LaserStatue.BP_LaserStatue_C|GetLaserColour LaserHit) (Variables|Default|GetSpawnReference) 0))
          (Transformation|AttachComponentToComponent _returnvalue (Variables|Character|GetMesh) "None" "KeepWorld" "KeepWorld" "KeepRelative" false)
          (Utilities|Array|Add (Variables|Default|GetLasersAttached) _returnvalue)
          (Utilities|Array|Add (Variables|/Game/Blueprints/LaserPuzzle/BP_LaserSpawn.BP_LaserSpawn_C|GetChildLasers (Variables|Default|GetSpawnReference)) _returnvalue)
          (return _returnvalue)
          (else
            (CallFunction|ClearAllLasers)))))))