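; Laser beam actor for a puzzle that stretches to whatever blocks it and can bounce in chains.
; Each tick it box-traces along its up vector, scales its mesh to the hit distance and compares the hit with the last actor.
; Target changes notify BPI_Lasers actors or remove following lasers through SpawnReference, while a steady reflector hit re-aims the bounce laser.
; Helpers set beam colour, append IDs and release statue targets on cancellation.
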(event EventBeginPlay
  (CallFunction|ChangeColour))

(event EventTick
  (params (DeltaSeconds :type Float%20%28single-precision%29))
  (CallFunction|SetEndPoint))

(fn ConstructionScript
  (|CallParentFunction))

(fn ChangeColour
  (bind _returnvalue (Rendering|Material|CreateDynamicMaterialInstance (Variables|Character|GetMesh) 0 "/Game/Materials/M_Laser.M_Laser" "None" :!class /Script/Engine.PrimitiveComponent))
  (Rendering|Material|SetVectorParameterValue _returnvalue "Colour" (Variables|Default|GetLaserColour) :!class /Script/Engine.MaterialInstanceDynamic))

(fn SetEndPoint
  (bind _returnvalue (Transformation|GetActorLocation))
  (bind _returnvalue_2 (Transformation|GetActorUpVector))
  (bind _returnvalue_3 (* _returnvalue_2 2.0))
  (bind _returnvalue_4 (+ _returnvalue _returnvalue_3))
  (bind _outhit (Collision|BoxTraceByChannel _returnvalue_4 (+ _returnvalue_4 (* _returnvalue_2 (LocalVariables|GetL-Range))) "0, 0, 0" "0, 0, 0" "TraceTypeQuery1" false 0 "None"))
  (bind _output_get (LocalVariables|SetL-HitInfo _outhit))
  (LocalVariables|SetL-HitActor (.HitActor (Collision|BreakHitResult _output_get)))
  (Transformation|SetWorldScale3D (Variables|Character|GetMesh) (Math|Vector|MakeVector 0.05 0.05 (Math|Float|SelectFloat (/ (+ (.Distance (Collision|BreakHitResult _output_get)) 1.0) 1e+02) (/ (LocalVariables|GetL-Range) 1e+02) (.bBlockingHit (Collision|BreakHitResult _output_get)))))
  (LocalVariables|GetL-HitActor
    (:then
      (Utilities|FlowControl|Sequence
        (:then_0
          (if (== (Variables|Default|GetLastHitActor) (LocalVariables|GetL-HitActor))
            (CallFunction|SameActorHit (LocalVariables|GetL-HitInfo))
            (else
              (CallFunction|DifferentActorHit (LocalVariables|GetL-HitActor) (LocalVariables|GetL-HitInfo)))))
        (:then_1
          (Variables|Default|SetLastHitActor (LocalVariables|GetL-HitActor)))))
    (:else
      (CallFunction|NothingHit (LocalVariables|GetL-HitInfo)))))

(fn UpdateID
  (params (AppendID :type String))
  (return (Utilities|String|Append (Variables|Default|GetLaserID) AppendID)))

(fn CancelTargetHit
  (params (Override :type Boolean))
  (Utilities|FlowControl|Sequence
    (:then_0
      (bind _lasthitactor (Variables|Default|GetLastHitActor)
        (:then
          (bind _asbp_laser_statue (Utilities|Casting|CastToBP_LaserStatue _lasthitactor))
          (if (and (Utilities|DoesObjectImplementInterface _asbp_laser_statue "/Game/Interfaces/BPI_Lasers.BPI_Lasers_C") (Utilities|Array|IsEmpty (Variables|/Game/Blueprints/LaserPuzzle/BP_LaserStatue.BP_LaserStatue_C|GetLasersAttached _asbp_laser_statue)))
            (Class|BPILasers|LaserBounce(Message) (Variables|Default|GetLastHitActor) self false)
            (else
              (Variables|/Game/Blueprints/LaserPuzzle/BP_LaserStatue.BP_LaserStatue_C|SetActive? _asbp_laser_statue false))))
        (:else)))
    (:then_1
      (if Override
        (return false)
        (else
          (Actor|DestroyActor)
          (return true))))))

(fn DifferentActorHit
  (params (HitActor :type Object%20Object%20Reference) (HitInformation :type Hit%20Result%20Structure))
  (Utilities|FlowControl|Sequence
    (:then_0
      (if (Utilities|DoesObjectImplementInterface (Variables|Default|GetLastHitActor) "/Game/Interfaces/BPI_Lasers.BPI_Lasers_C")
        (Default|RemoveFollowingLasers (Variables|Default|GetSpawnReference) self)))
    (:then_1
      (if (Utilities|DoesObjectImplementInterface HitActor "/Game/Interfaces/BPI_Lasers.BPI_Lasers_C")
        (bind _newlaser (Class|BPILasers|LaserBounce(Message) HitActor self true HitInformation))
        (Variables|Default|SetBounce%20Laser _newlaser)))))

(fn SameActorHit
  (params (Hit :type Hit%20Result%20Structure%20%28by%20ref%29))
  (bind (_bblockinghit _binitialoverlap _time _distance _location _impactpoint _normal _impactnormal _physmat _hitactor _hitcomponent _hitbonename _bonename _hititem _elementindex _faceindex _tracestart) (Collision|BreakHitResult Hit))
  (bind _asbp_laser_reflector (Utilities|Casting|CastToBP_LaserReflector (Variables|Default|GetLastHitActor)))
  (Transformation|SetActorLocation (Variables|Default|GetBounce%20Laser) (.ImpactPoint (Collision|BreakHitResult Hit)) false false)
  (Transformation|SetActorRotation (Variables|Default|GetBounce%20Laser) (Default|CalculateRotation _asbp_laser_reflector _impactpoint _impactnormal _tracestart)))

(fn NothingHit
  (params (HitInformation :type Hit%20Result%20Structure))
  (Utilities|FlowControl|Sequence
    (:then_0
      (bind _lasthitactor (Variables|Default|GetLastHitActor)
        (:then
          (if (Utilities|DoesObjectImplementInterface _lasthitactor "/Game/Interfaces/BPI_Lasers.BPI_Lasers_C")
            (Class|BPILasers|LaserBounce(Message) (Variables|Default|GetLastHitActor) self false HitInformation)))
        (:else)))
    (:then_1
      (Variables|Default|SetLastHitActor 0)
      (Variables|Default|SetBounce%20Laser 0))))