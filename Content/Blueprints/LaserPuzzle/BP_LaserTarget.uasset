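; BP_LaserTarget is a laser puzzle target that shows whether a laser is hitting it.
; LaserBounce stores the hit response as its Active state and passes the laser's colour to PuzzleComplete.
; PuzzleComplete creates a dynamic instance of M_Solid on the mesh on each call, tinting it the laser colour when active or dark grey otherwise.
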(event EventBeginPlay)

(fn ConstructionScript
  (|CallParentFunction))

(fn PuzzleComplete
  (params (Colour :type Linear%20Color%20Structure))
  (bind _returnvalue (Rendering|Material|CreateDynamicMaterialInstance (Variables|Character|GetMesh) 0 "/Game/LevelPrototyping/Materials/M_Solid.M_Solid" "None" :!class /Script/Engine.PrimitiveComponent))
  (Rendering|Material|SetVectorParameterValue _returnvalue "Base Color" (Math|Color|SelectColor Colour "(R=0.203125,G=0.203125,B=0.203125,A=1.000000)" (Variables|Default|GetActive?)) :!class /Script/Engine.MaterialInstanceDynamic))

(fn LaserBounce
  (params (LaserHit :type BP%20Laser%20Object%20Reference) (HitResponse :type Boolean) (HitInformation :type Hit%20Result%20Structure))
  (Variables|Default|SetActive? HitResponse)
  (CallFunction|PuzzleComplete (Variables|/Game/Blueprints/LaserPuzzle/BP_LaserStatue.BP_LaserStatue_C|GetLaserColour LaserHit))
  (return 0))