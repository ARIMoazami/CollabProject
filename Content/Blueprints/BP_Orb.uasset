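; BP_Orb is an orb whose material reflects one of three dimensions and a cooldown state.
; Construction creates a dynamic instance of MI_Dimension on the Orb, which every event drives.
; Each dimension event runs a timeline blending Inner Colour from the stored colour to red, blue or grey, saving the result on finish.
; Cooldown resets FresnelSubtraction, then animates it from CurrentCooldown to a low value.
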(event Custom|OrbDimension3
  (bind _alpha (Timeline|Timeline_0 PlayFromStart)
    (:Update
      (Rendering|Material|SetVectorParameterValue (Variables|Default|GetOrbMaterial) "Inner Colour" (Math|Color|Lerp(LinearColor) (Variables|Default|GetCurrentOrbColour) "(R=0.300000,G=0.300000,B=0.300000,A=1.000000)" _alpha) :!class /Script/Engine.MaterialInstanceDynamic))
    (:Finished
      (Variables|Default|SetCurrentOrbColour (Math|Color|Lerp(LinearColor) (Variables|Default|GetCurrentOrbColour) "(R=0.300000,G=0.300000,B=0.300000,A=1.000000)" _alpha)))))

(event Custom|OrbDimension1
  (bind _alpha (Timeline|ColourSwitch PlayFromStart)
    (:Update
      (Rendering|Material|SetVectorParameterValue (Variables|Default|GetOrbMaterial) "Inner Colour" (Math|Color|Lerp(LinearColor) (Variables|Default|GetCurrentOrbColour) "(R=0.730000,G=0.000000,B=0.000000,A=1.000000)" _alpha) :!class /Script/Engine.MaterialInstanceDynamic))
    (:Finished
      (Variables|Default|SetCurrentOrbColour (Math|Color|Lerp(LinearColor) (Variables|Default|GetCurrentOrbColour) "(R=0.730000,G=0.000000,B=0.000000,A=1.000000)" _alpha)))))

(event Custom|Cooldown
  (Rendering|Material|SetScalarParameterValue (Variables|Default|GetOrbMaterial) "FresnelSubtraction" 1.0 :!class /Script/Engine.MaterialInstanceDynamic)
  (bind _alpha (Timeline|Timeline_1 PlayFromStart)
    (:Update
      (Rendering|Material|SetScalarParameterValue (Variables|Default|GetOrbMaterial) "FresnelSubtraction" (Math|Float|Lerp (Variables|Default|GetCurrentCooldown) 0.1 _alpha) :!class /Script/Engine.MaterialInstanceDynamic))))

(event Custom|OrbDimension2
  (bind _alpha (Timeline|Timeline PlayFromStart)
    (:Update
      (Rendering|Material|SetVectorParameterValue (Variables|Default|GetOrbMaterial) "Inner Colour" (Math|Color|Lerp(LinearColor) (Variables|Default|GetCurrentOrbColour) "(R=0.000000,G=0.100000,B=0.300000,A=1.000000)" _alpha) :!class /Script/Engine.MaterialInstanceDynamic))
    (:Finished
      (Variables|Default|SetCurrentOrbColour (Math|Color|Lerp(LinearColor) (Variables|Default|GetCurrentOrbColour) "(R=0.000000,G=0.100000,B=0.300000,A=1.000000)" _alpha)))))

(fn ConstructionScript
  (bind _returnvalue (Rendering|Material|CreateDynamicMaterialInstance "/Game/Character/Asset/MI_Dimension.MI_Dimension" "None" "None" :!class /Script/Engine.KismetMaterialLibrary))
  (bind _output_get (Variables|Default|SetOrbMaterial _returnvalue))
  (Rendering|Material|SetMaterial (Variables|Default|GetOrb) 0 _output_get))