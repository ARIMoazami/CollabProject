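; Interactable statue that turns 45 degrees in yaw on each Interact and reports to a linked Portal, likely as part of a rotation puzzle.
; Interact resets the rotation once yaw reaches a full turn, then stores start and target angles for the Rotation timeline.
; Each timeline update lerps the statue's relative yaw and calls StatueCheck on the Portal.
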(event OnComponentBeginOverlap(Box)
  (params (OverlappedComponent :type Primitive%20Component%20Object%20Reference) (OtherActor :type Actor%20Object%20Reference) (OtherComp :type Primitive%20Component%20Object%20Reference) (OtherBodyIndex :type Integer) (bFromSweep :type Boolean) (SweepResult :type Hit%20Result%20Structure%20%28by%20ref%29)))

(event EventInteract
  (params (Player :type BP%20First%20Person%20Character%20Object%20Reference))
  (if (>= (.yaw (Variables|/Script/Engine.SceneComponent|GetRelativeRotation (Variables|Default|GetStatue))) 3.6e+02)
    (Transformation|SetRelativeRotation (Variables|Default|GetStatue) (Math|Rotator|MakeRotator 0.0 0.0 0.0) false false))
  (bind _output_get (Variables|Default|SetOldRotation (.yaw (Variables|/Script/Engine.SceneComponent|GetRelativeRotation (Variables|Default|GetStatue)))))
  (bind _output_get_2 (Variables|Default|SetNewRotation (+ (.yaw (Variables|/Script/Engine.SceneComponent|GetRelativeRotation (Variables|Default|GetStatue))) 45.0)))
  (bind _alpha (Timeline|Rotation PlayFromStart)
    (:Update
      (Transformation|SetRelativeRotation (Variables|Default|GetStatue) (Math|Rotator|MakeRotator 0.0 0.0 (Math|Float|Lerp _output_get _output_get_2 _alpha)) false false)
      (Default|StatueCheck (Variables|Default|Getportal) (Variables|Default|GetValue)))))

(fn ConstructionScript)