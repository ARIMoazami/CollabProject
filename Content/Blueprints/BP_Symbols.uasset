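; BP_Symbols is a Blueprint that gives its Symbol component one of three random looks when play begins.
; BeginPlay calls RandomNumber, which stores a random integer in SymbolValue and returns it.
; A switch on that value sets the component's first material slot to the G, B or R variant of M_Symbols.
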(event EventBeginPlay
  (switch int (CallFunction|RandomNumber)
    (:0
      (Rendering|Material|SetMaterial (Variables|Default|GetSymbol) 0 "/Game/Materials/M_SymbolsG.M_SymbolsG"))
    (:1
      (Rendering|Material|SetMaterial (Variables|Default|GetSymbol) 0 "/Game/Materials/M_SymbolsB.M_SymbolsB"))
    (:2
      (Rendering|Material|SetMaterial (Variables|Default|GetSymbol) 0 "/Game/Materials/M_SymbolsR.M_SymbolsR"))))

(fn ConstructionScript)

(fn RandomNumber
  (bind _output_get (Variables|Default|SetSymbolValue (Math|Random|RandomIntegerinRange 0 2)))
  (return _output_get))