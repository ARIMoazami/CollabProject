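; Interactable gyro pedestal puzzle Blueprint that toggles the player's gyro state and item.
; Interact flip-flops between setting GyroActive with ApplyItem and clearing it with RemoveItem, each playing a timeline that lerps the cube's dissolve in opposite directions.
; A dynamic material instance created in the construction script drives the dissolve, and the stored value updates when each timeline finishes.
; A box overlap toggles the pedestal's hover outline for the player character.
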(event OnComponentBeginOverlap(Box)
  (params (OverlappedComponent :type Primitive%20Component%20Object%20Reference) (OtherActor :type Actor%20Object%20Reference) (OtherComp :type Primitive%20Component%20Object%20Reference) (OtherBodyIndex :type Integer) (bFromSweep :type Boolean) (SweepResult :type Hit%20Result%20Structure%20%28by%20ref%29))
  (if (== OtherActor (Game|GetPlayerCharacter 0))
    (CallFunction|ObjectHoveredOutline true (Variables|Default|GetPedastal))))

(event OnComponentEndOverlap(Box)
  (params (OverlappedComponent :type Primitive%20Component%20Object%20Reference) (OtherActor :type Actor%20Object%20Reference) (OtherComp :type Primitive%20Component%20Object%20Reference) (OtherBodyIndex :type Integer))
  (if (== OtherActor (Game|GetPlayerCharacter 0))
    (CallFunction|ObjectHoveredOutline false (Variables|Default|GetPedastal))))

(event EventInteract
  (params (Player :type BP%20First%20Person%20Character%20Object%20Reference))
  (Utilities|FlowControl|FlipFlop
    (:A
      (bind _alpha (Timeline|Timeline PlayFromStart)
        (:Update
          (Rendering|Material|SetScalarParameterValue (Variables|Default|GetDissolveMaterial) "Dissolve Amount" (Math|Float|Lerp (Variables|Default|GetCurrentDissolveValue) -1.0 _alpha) :!class /Script/Engine.MaterialInstanceDynamic)
          (Variables|/Game/FirstPerson/Blueprints/BP_FirstPersonCharacter.BP_FirstPersonCharacter_C|SetGyroActive? Player true)
          (Default|ApplyItem Player))
        (:Finished
          (Variables|Default|SetCurrentDissolveValue (Math|Float|Lerp (Variables|Default|GetCurrentDissolveValue) -1.0 _alpha)))))
    (:B
      (Default|RemoveItem Player)
      (bind _alpha_2 (Timeline|Timeline_0 PlayFromStart)
        (:Update
          (Rendering|Material|SetScalarParameterValue (Variables|Default|GetDissolveMaterial) "Dissolve Amount" (Math|Float|Lerp (Variables|Default|GetCurrentDissolveValue) 1.0 _alpha_2) :!class /Script/Engine.MaterialInstanceDynamic)
          (Variables|/Game/FirstPerson/Blueprints/BP_FirstPersonCharacter.BP_FirstPersonCharacter_C|SetGyroActive? Player false))
        (:Finished
          (Variables|Default|SetCurrentDissolveValue (Math|Float|Lerp (Variables|Default|GetCurrentDissolveValue) 1.0 _alpha_2)))))))

(fn ConstructionScript
  (bind _returnvalue (Rendering|Material|CreateDynamicMaterialInstance (Variables|Default|GetCube) 0 "/Game/Materials/MI_DissolveGyro.MI_DissolveGyro" "None" :!class /Script/Engine.PrimitiveComponent))
  (Variables|Default|SetDissolveMaterial _returnvalue))