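; Puzzle symbol switch that cycles through green, blue and red symbol materials as one element of a code combination.
; Overlapping the box toggles an outline on the cube for the player character.
; Interacting advances the symbol, has CodeManager check the combination and plays a sound, with a short lockout between presses.
; BeginPlay also runs the switch, and the local CheckCombination function is empty.
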(event OnComponentBeginOverlap(Box)
  (params (OverlappedComponent :type Primitive%20Component%20Object%20Reference) (OtherActor :type Actor%20Object%20Reference) (OtherComp :type Primitive%20Component%20Object%20Reference) (OtherBodyIndex :type Integer) (bFromSweep :type Boolean) (SweepResult :type Hit%20Result%20Structure%20%28by%20ref%29))
  (if (== OtherActor (Game|GetPlayerCharacter 0))
    (CallFunction|ObjectHoveredOutline true (Variables|Default|GetCube))))

(event OnComponentEndOverlap(Box)
  (params (OverlappedComponent :type Primitive%20Component%20Object%20Reference) (OtherActor :type Actor%20Object%20Reference) (OtherComp :type Primitive%20Component%20Object%20Reference) (OtherBodyIndex :type Integer))
  (if (== OtherActor (Game|GetPlayerCharacter 0))
    (CallFunction|ObjectHoveredOutline false (Variables|Default|GetCube))))

(event EventInteract
  (params (Player :type BP%20First%20Person%20Character%20Object%20Reference))
  (if (Variables|Default|GetActive?)
    (Variables|Default|SetActive? false)
    (CallFunction|SwitchSymbol (Variables|Default|GetSymbol%20Number))
    (Default|CheckCombination (Variables|Default|GetCodeManager))
    (Audio|PlaySound2D "/Game/Sounds/CodeSwitch.CodeSwitch" 1.0 1.0 0.0 0 0)
    (Utilities|FlowControl|Delay 1.0)
    (Variables|Default|SetActive? true)))

(event EventBeginPlay
  (CallFunction|SwitchSymbol (Variables|Default|GetSymbol%20Number)))

(fn ConstructionScript)

(fn SwitchSymbol
  (params (SymbolNumber :type Integer))
  (bind _result (Math|Integer|IncrementInt SymbolNumber)
    (:%20%20
      (if (> _result 2)
        (Variables|Default|SetSymbol%20Number 0)
        (else
          (Variables|Default|SetSymbol%20Number _result)))
      (switch int (Variables|Default|GetSymbol%20Number)
        (:0
          (Rendering|Material|SetMaterial (Variables|Default|GetSymbol) 0 "/Game/Materials/M_SymbolsGreen.M_SymbolsGreen"))
        (:1
          (Rendering|Material|SetMaterial (Variables|Default|GetSymbol) 0 "/Game/Materials/M_SymbolsBlue.M_SymbolsBlue"))
        (:2
          (Rendering|Material|SetMaterial (Variables|Default|GetSymbol) 0 "/Game/Materials/M_SymbolsRed.M_SymbolsRed"))))))

(fn CheckCombination)