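; BP_CubePlate is a puzzle pressure plate that signals a linked gate when a rolling crate or the player enters its trigger box.
; A BP_CrateRolling overlap switches two linked cables to the lit material and calls OnPlate on the gate.
; A BP_FirstPersonCharacter overlap calls OnPlate without changing the cables.
; End overlap does nothing, so the plate never reverts the cables or notifies the gate on exit.
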(event OnComponentBeginOverlap(Box)
  (params (OverlappedComponent :type Primitive%20Component%20Object%20Reference) (OtherActor :type Actor%20Object%20Reference) (OtherComp :type Primitive%20Component%20Object%20Reference) (OtherBodyIndex :type Integer) (bFromSweep :type Boolean) (SweepResult :type Hit%20Result%20Structure%20%28by%20ref%29))
  (if (== OtherActor (.AsBP%20Crate%20Rolling (Utilities|Casting|CastToBP_CrateRolling OtherActor)))
    (Rendering|Material|SetMaterial (Variables|/Script/CableComponent.CableActor|GetCableComponent (Variables|Default|GetCable1)) 0 "/Game/Materials/M_CableOn.M_CableOn")
    (Default|OnPlate (Variables|Default|GetGate))
    (elif (== OtherActor (.AsBP%20First%20Person%20Character (Utilities|Casting|CastToBP_FirstPersonCharacter OtherActor)))
      (Default|OnPlate (Variables|Default|GetGate)))))

(event OnComponentEndOverlap(Box)
  (params (OverlappedComponent :type Primitive%20Component%20Object%20Reference) (OtherActor :type Actor%20Object%20Reference) (OtherComp :type Primitive%20Component%20Object%20Reference) (OtherBodyIndex :type Integer)))

(fn ConstructionScript)