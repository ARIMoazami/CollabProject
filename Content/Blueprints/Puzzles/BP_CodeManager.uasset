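; BP_CodeManager is a puzzle actor that checks a two-symbol code and ends the game when it is solved.
; CheckCombination compares each Symbol actor's SymbolValue with the SymbolNumber of its matching CODE reference.
; On a match it plays a success sound, calls End on the first-person character's PlayerUI, then opens the main menu level after a short delay.
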(event Custom|CheckCombination
  (if (and (== (Variables|/Game/Blueprints/BP_Symbols.BP_Symbols_C|GetSymbolValue (Variables|Default|GetSymbol1)) (Variables|/Game/Blueprints/Puzzles/BP_SymbolCode.BP_SymbolCode_C|GetSymbol%20Number (Variables|Default|GetSymbol1%20CODE))) (== (Variables|/Game/Blueprints/BP_Symbols.BP_Symbols_C|GetSymbolValue (Variables|Default|GetSymbol2)) (Variables|/Game/Blueprints/Puzzles/BP_SymbolCode.BP_SymbolCode_C|GetSymbol%20Number (Variables|Default|GetSymbol2%20CODE))))
    (Audio|PlaySound2D "/Game/Sounds/730116__riley_garinger__music_consonant-oneshot-somber-warm-bright.730116__riley_garinger__music_consonant-oneshot-somber-warm-bright" 1.0 1.0 0.0 0 0)
    (bind _asbp_first_person_character (Utilities|Casting|CastToBP_FirstPersonCharacter (Game|GetPlayerCharacter 0)))
    (Default|End (Variables|/Game/FirstPerson/Blueprints/BP_FirstPersonCharacter.BP_FirstPersonCharacter_C|GetPlayerUI _asbp_first_person_character))
    (Utilities|FlowControl|Delay 4.0)
    (Game|OpenLevel(byObjectReference) "/Game/Levels/L_MainMenu.L_MainMenu")))

(event EventBeginPlay)

(fn ConstructionScript)