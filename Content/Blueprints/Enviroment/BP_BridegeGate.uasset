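; A bridge gate whose wall dissolves in stages as pressure plates are occupied, opening fully with two.
; The construction script creates a dynamic dissolve material on the wall, which timelines animate from a tracked current value.
; OnPlate and OffPlate adjust a plate count to pick the dissolve target, until a completed opening disables collision and locks the plates.
; A separate OpenGate event dissolves the wall and disables collision regardless of plate count.
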(event Custom|OffPlate
  (if (not (Variables|Default|GetPlateLocked?))
    (bind _result (Math|Integer|DecrementInt (Variables|Default|GetPlateCount))
      (:%20%20
        (if (== _result 0)
          (bind _alpha (Timeline|Timeline_1 PlayFromStart)
            (:Update
              (Rendering|Material|SetScalarParameterValue (Variables|Default|GetDissolveMaterial) "Dissolve Amount" (Math|Float|Lerp (Variables|Default|GetCurrentDissolveValue) 1.0 _alpha) :!class /Script/Engine.MaterialInstanceDynamic)
              (Variables|Default|SetCurrentDissolveValue (Math|Float|Lerp (Variables|Default|GetCurrentDissolveValue) 1.0 _alpha))))
          (elif (== _result 1)
            (bind _alpha_2 (Timeline|Timeline_2 PlayFromStart)
              (:Update
                (Rendering|Material|SetScalarParameterValue (Variables|Default|GetDissolveMaterial) "Dissolve Amount" (Math|Float|Lerp (Variables|Default|GetCurrentDissolveValue) 0.4 _alpha_2) :!class /Script/Engine.MaterialInstanceDynamic)
                (Variables|Default|SetCurrentDissolveValue (Math|Float|Lerp (Variables|Default|GetCurrentDissolveValue) 0.4 _alpha_2))))))))))

(event Custom|OnPlate
  (bind _result (Math|Integer|IncrementInt (Variables|Default|GetPlateCount))
    (:%20%20
      (if (== _result 2)
        (bind _alpha (Timeline|Timeline PlayFromStart)
          (:Update
            (Rendering|Material|SetScalarParameterValue (Variables|Default|GetDissolveMaterial) "Dissolve Amount" (Math|Float|Lerp (Variables|Default|GetCurrentDissolveValue) -1.0 _alpha) :!class /Script/Engine.MaterialInstanceDynamic))
          (:Finished
            (Variables|Default|SetCurrentDissolveValue (Math|Float|Lerp (Variables|Default|GetCurrentDissolveValue) -1.0 _alpha))
            (Collision|SetCollisionEnabled (Variables|Default|GetWall) "NoCollision")
            (Variables|Default|SetPlateLocked? true)))
        (elif (== _result 1)
          (bind _alpha_2 (Timeline|Timeline_0 PlayFromStart)
            (:Update
              (Rendering|Material|SetScalarParameterValue (Variables|Default|GetDissolveMaterial) "Dissolve Amount" (Math|Float|Lerp (Variables|Default|GetCurrentDissolveValue) 0.4 _alpha_2) :!class /Script/Engine.MaterialInstanceDynamic))
            (:Finished
              (Variables|Default|SetCurrentDissolveValue (Math|Float|Lerp (Variables|Default|GetCurrentDissolveValue) 0.4 _alpha_2)))))))))

(event Custom|OpenGate
  (bind _alpha (Timeline|Timeline_3 PlayFromStart)
    (:Update
      (Rendering|Material|SetScalarParameterValue (Variables|Default|GetDissolveMaterial) "Dissolve Amount" (Math|Float|Lerp (Variables|Default|GetCurrentDissolveValue) -1.0 _alpha) :!class /Script/Engine.MaterialInstanceDynamic))
    (:Finished
      (Variables|Default|SetCurrentDissolveValue (Math|Float|Lerp (Variables|Default|GetCurrentDissolveValue) -1.0 _alpha))
      (Collision|SetCollisionEnabled (Variables|Default|GetWall) "NoCollision"))))

(fn ConstructionScript
  (bind _returnvalue (Rendering|Material|CreateDynamicMaterialInstance (Variables|Default|GetWall) 0 "/Game/Materials/MI_Dissolve.MI_Dissolve" "None" :!class /Script/Engine.PrimitiveComponent))
  (Variables|Default|SetDissolveMaterial _returnvalue))